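; BP_ScreenshotTool is a camera-based utility that captures high-resolution HDR screenshots from its own view.
; Ticking TickBoxToCapture makes the Construction Script call CaptureScreenshot and then clear the flag, so the checkbox acts as a button.
; The capture matches the camera's aspect ratio to Resolution, then saves to Filename at Resolution scaled by ResolutionMultiplier.
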(event `Capture Screenshot`
  (bind _resolution (`self.Resolution`))
  (bind (_x _y) (`KismetMathLibrary.BreakVector2D` _resolution))
  (bind (_x_2 _y_2) (`KismetMathLibrary.BreakVector2D` (* _resolution (`self.ResolutionMultiplier`))))
  (`CameraComponent.SetAspectRatio` (`self.CameraComponent`) (/ _x _y))
  (`AutomationBlueprintFunctionLibrary.TakeHighResScreenshot` (`KismetMathLibrary.FTrunc` _x_2) (`KismetMathLibrary.FTrunc` _y_2) (`self.Filename`) self false true "High"))

(fn `UserConstructionScript`
  (if (`self.Tick box to capture!`)
    (`self.Capture Screenshot`)
    (set `self.Tick box to capture!` false)))